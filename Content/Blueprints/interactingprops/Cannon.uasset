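; Interactive cannon prop that fires a single shot when a torch item touches its fuse trigger box.
; On torch overlap it sets a one-time Fired flag, spawns spark and explosion effects, and spawns a Shootball from the "boom" socket along the actor's forward vector.
; A second box shows an on-screen hint to light the fuse when a player character enters while unfired, and removes it on exit.
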(event `self.Box.OnComponentBeginOverlap`
  (params (OverlappedComponent :type "PrimitiveComponent Object Reference") (OtherActor :type "Actor Object Reference") (OtherComp :type "PrimitiveComponent Object Reference") (OtherBodyIndex :type Integer) (bFromSweep :type Boolean) (SweepResult :type "HitResult Structure (by ref)"))
  (bind _returnvalue (`SceneComponent.GetSocketLocation` (`self.StaticMesh`) "boom"))
  (if (not (`self.Fired`))
    (cast `/Game/Blueprints/Inventory/Item_torch` OtherActor)
    (set `self.Fired` true)
    (`GameplayStatics.SpawnEmitterAtLocation` "/Game/FX/Particles/P_Sparks.P_Sparks" (0.0 0.0 0.0) (struct) (1.0 1.0 1.0) false)
    (`GameplayStatics.SpawnEmitterAtLocation` "/Game/FX/Particles/P_Explosion.P_Explosion" _returnvalue)
    (`|SpawnActorFromClass` "/Game/Blueprints/projectiles/shootball.shootball_C" (`KismetMathLibrary.MakeTransform` _returnvalue (`KismetMathLibrary.Conv_VectorToRotator` (`self.GetActorForwardVector` self))) "Undefined" "OverrideRootScale" null null)))

(event `self.Box1.OnComponentBeginOverlap`
  (params (OverlappedComponent :type "PrimitiveComponent Object Reference") (OtherActor :type "Actor Object Reference") (OtherComp :type "PrimitiveComponent Object Reference") (OtherBodyIndex :type Integer) (bFromSweep :type Boolean) (SweepResult :type "HitResult Structure (by ref)"))
  (if (not (`self.Fired`))
    (bind _asbase_character (cast `/Game/Blueprints/characters/BaseCharacter` OtherActor))
    (`/Engine/EditorBlueprintResources/StandardMacros.IsValid` (`self.ScrenRef`)
      (:`Is Not Valid`
        (bind _asmc_player_controller (cast `/Game/Blueprints/game/MC_PlayerController` (`Pawn.GetController` _asbase_character)))
        (bind _returnvalue (`|CreateWidget` "/Game/UI/ScreenMessage.ScreenMessage_C" _asmc_player_controller "Lit the fuse with a torch to shoot"))
        (bind _output_get (set `self.ScrenRef` _returnvalue))
        (`UserWidget.AddToViewport` _output_get 0)))))

(event `self.Box1.OnComponentEndOverlap`
  (params (OverlappedComponent :type "PrimitiveComponent Object Reference") (OtherActor :type "Actor Object Reference") (OtherComp :type "PrimitiveComponent Object Reference") (OtherBodyIndex :type Integer))
  (bind _screnref (`self.ScrenRef`))
  (`/Engine/EditorBlueprintResources/StandardMacros.IsValid` _screnref
    (:`Is Valid`
      (`Widget.RemoveFromParent` _screnref)
      (set `self.ScrenRef` null))))

(fn `UserConstructionScript`)