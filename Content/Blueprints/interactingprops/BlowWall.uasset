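; BlowWall is a destructible wall prop that breaks when a shootball actor enters its box trigger.
; On that hit it spawns a scaled-up explosion emitter at its root, spawns a Blowall_Debris actor at a hardcoded world transform, then destroys itself.
; When a BaseCharacter overlaps the box instead, it shows a single ScreenMessage widget through its MC_PlayerController and removes it on end overlap.
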(event `self.Box.OnComponentBeginOverlap`
  (params (OverlappedComponent :type "PrimitiveComponent Object Reference") (OtherActor :type "Actor Object Reference") (OtherComp :type "PrimitiveComponent Object Reference") (OtherBodyIndex :type Integer) (bFromSweep :type Boolean) (SweepResult :type "HitResult Structure (by ref)"))
  (cast `/Game/Blueprints/projectiles/shootball` OtherActor
    (:`then`
      (`GameplayStatics.SpawnEmitterAtLocation` "/Game/FX/Particles/P_Explosion.P_Explosion" (`SceneComponent.K2_GetComponentLocation` (`self.DefaultSceneRoot`)) (struct) (5.0 5.0 5.0))
      (`|SpawnActorFromClass` "/Game/Blueprints/interactingprops/Blowall_Debris.Blowall_Debris_C" (`KismetMathLibrary.MakeTransform` (-9606.90918 66722.421875 -6191.541992)) "AdjustIfPossibleButAlwaysSpawn" "OverrideRootScale" null null)
      (`self.K2_DestroyActor`))
    (:`CastFailed`
      (`/Engine/EditorBlueprintResources/StandardMacros.IsValid` (`self.screenmessageref`)
        (:`Is Not Valid`
          (bind _asbase_character (cast `/Game/Blueprints/characters/BaseCharacter` OtherActor))
          (bind _asmc_player_controller (cast `/Game/Blueprints/game/MC_PlayerController` (`Pawn.GetController` _asbase_character)))
          (bind _returnvalue (`|CreateWidget` "/Game/UI/ScreenMessage.ScreenMessage_C" _asmc_player_controller (`self.Screen Message`)))
          (bind _output_get (set `self.screenmessageref` _returnvalue))
          (`UserWidget.AddToViewport` _output_get 0))))))

(event `self.Box.OnComponentEndOverlap`
  (params (OverlappedComponent :type "PrimitiveComponent Object Reference") (OtherActor :type "Actor Object Reference") (OtherComp :type "PrimitiveComponent Object Reference") (OtherBodyIndex :type Integer))
  (bind _screenmessageref (`self.screenmessageref`))
  (cast `/Game/Blueprints/characters/BaseCharacter` OtherActor)
  (`/Engine/EditorBlueprintResources/StandardMacros.IsValid` _screenmessageref
    (:`Is Valid`
      (`Widget.RemoveFromParent` _screenmessageref)
      (set `self.screenmessageref` null))))

(fn `UserConstructionScript`)