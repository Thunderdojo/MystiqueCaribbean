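; Sack is a "ship sack" pickup actor that a BaseCharacter can find and carry.
; Overlapping its capsule shows a ScreenMessage widget to that character's MC_PlayerController, removed after a short delay or when the overlap ends.
; On InterAct it disables its collision, stores itself in the character's SackRef and snaps onto the "Sacky" socket of the character's mesh.
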(event `self.Capsule.OnComponentBeginOverlap`
  (params (OverlappedComponent :type "PrimitiveComponent Object Reference") (OtherActor :type "Actor Object Reference") (OtherComp :type "PrimitiveComponent Object Reference") (OtherBodyIndex :type Integer) (bFromSweep :type Boolean) (SweepResult :type "HitResult Structure (by ref)"))
  (bind _screenmref (`self.ScreenmRef`))
  (bind _asbase_character (cast `/Game/Blueprints/characters/BaseCharacter` OtherActor))
  (`/Engine/EditorBlueprintResources/StandardMacros.IsValid` (`self.ScreenmRef`)
    (:`Is Not Valid`
      (bind _asmc_player_controller (cast `/Game/Blueprints/game/MC_PlayerController` (`Pawn.GetController` _asbase_character)))
      (bind _returnvalue (`|CreateWidget` "/Game/UI/ScreenMessage.ScreenMessage_C" _asmc_player_controller "You found a ship sack" 1))
      (bind _output_get (set `self.ScreenmRef` _returnvalue))
      (`UserWidget.AddToViewport` _output_get 0)
      (`KismetSystemLibrary.Delay` 1.5)
      (`/Engine/EditorBlueprintResources/StandardMacros.IsValid` _screenmref
        (:`Is Valid`
          (`Widget.RemoveFromParent` _screenmref)
          (set `self.ScreenmRef` null))))))

(event `self.Capsule.OnComponentEndOverlap`
  (params (OverlappedComponent :type "PrimitiveComponent Object Reference") (OtherActor :type "Actor Object Reference") (OtherComp :type "PrimitiveComponent Object Reference") (OtherBodyIndex :type Integer))
  (bind _screenmref (`self.ScreenmRef`))
  (`/Engine/EditorBlueprintResources/StandardMacros.IsValid` _screenmref
    (:`Is Valid`
      (`Widget.RemoveFromParent` _screenmref)
      (set `self.ScreenmRef` null))))

(event `/Game/Blueprints/interfaces/E_InterFace.InterAct`
  (params (Interactor :type "Actor Object Reference"))
  (bind _asbase_character (cast `/Game/Blueprints/characters/BaseCharacter` Interactor :!pure true))
  (`self.SetActorEnableCollision` self false)
  (set `/Game/Blueprints/characters/BaseCharacter.SackRef` self _asbase_character)
  (`self.K2_AttachToComponent` self (`Character.Mesh` _asbase_character) "Sacky" "SnapToTarget" "SnapToTarget" "SnapToTarget" true))

(fn `UserConstructionScript`)