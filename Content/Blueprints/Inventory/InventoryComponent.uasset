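; Inventory component that toggles a player's inventory or sack screen and holds an array of item slots.
; ToggleUI hands inventories named "Sack" to ToggleSack; each creates or removes its widget, switching mouse cursor and input mode.
; Widgets receive this component and its name, not the passed-in inventory.
; AddToInventory is unfinished: it writes to every empty slot for non-stackable items with no value wired, and stacking logic is unconnected.
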(event `self.ReceiveBeginPlay`)

(fn `AddToInventory`
  (params (NewParam :type "/Game/Blueprints/Inventory/ItemStruct Structure"))
  (for (_array_element _array_index) (`self.InventorySlots`)
    (if (`.CanBeStacked?_31_2D02D0554440DA45BF1208AA806FDF57` (break `/Game/Blueprints/Inventory/ItemStruct` NewParam))
      _
      (elif (== (`.Class_14_0D2681914B7F4011C3F7A5A9D17D87E8` (break `/Game/Blueprints/Inventory/ItemStruct` _array_element)) null)
        (`KismetArrayLibrary.Array_Set` (`self.InventorySlots`) _array_index)))))

(fn `ToggleSack`
  (params (input :type "/Game/Blueprints/Inventory/InventoryComponent Object Reference"))
  (bind _returnvalue (`GameplayStatics.GetPlayerController` 0))
  (bind _returnvalue_2 (`GameplayStatics.GetPlayerController` 0))
  (bind _output_get (set `self.InventoryRef` input))
  (`/Engine/EditorBlueprintResources/StandardMacros.IsValid` _output_get
    (:`Is Valid`
      (`/Engine/EditorBlueprintResources/StandardMacros.IsValid` (`self.SackW`)
        (:`Is Valid`
          (`Widget.RemoveFromParent` (`self.SackW`))
          (set `self.SackW` null)
          (set `PlayerController.bShowMouseCursor` false _returnvalue_2)
          (`WidgetBlueprintLibrary.SetInputMode_GameOnly` _returnvalue_2)
          (set `self.InventoryRef` null)
          (return))
        (:`Is Not Valid`
          (bind _asmc_player_controller (cast `/Game/Blueprints/game/MC_PlayerController` (`GameplayStatics.GetPlayerController` 0)))
          (bind _returnvalue_3 (`|CreateWidget` "/Game/Blueprints/Inventory/InventoryUI/SackWidget.SackWidget_C" _asmc_player_controller self (`self.InventoryName`)))
          (bind _output_get_2 (set `self.SackW` _returnvalue_3))
          (`UserWidget.AddToViewport` _output_get_2 0)
          (set `PlayerController.bShowMouseCursor` true _returnvalue)
          (`WidgetBlueprintLibrary.SetInputMode_GameAndUIEx` _returnvalue null)
          (return))))))

(fn `ToggleUI`
  (params (iventoryref :type "/Game/Blueprints/Inventory/InventoryComponent Object Reference"))
  (bind _returnvalue (`GameplayStatics.GetPlayerController` 0))
  (bind _returnvalue_2 (`GameplayStatics.GetPlayerController` 0))
  (bind _output_get (set `self.InventoryRef` iventoryref))
  (`/Engine/EditorBlueprintResources/StandardMacros.IsValid` _output_get
    (:`Is Valid`
      (if (`KismetTextLibrary.EqualEqual_TextText` (`/Game/Blueprints/Inventory/InventoryComponent.InventoryName` (`self.InventoryRef`)) "Sack")
        (`self.ToggleSack` (`self.InventoryRef`))
        (else
          (`/Engine/EditorBlueprintResources/StandardMacros.IsValid` (`self.InventoryW`)
            (:`Is Valid`
              (`Widget.RemoveFromParent` (`self.InventoryW`))
              (set `self.InventoryW` null)
              (set `self.InventoryRef` null)
              (set `PlayerController.bShowMouseCursor` false _returnvalue)
              (`WidgetBlueprintLibrary.SetInputMode_GameOnly` _returnvalue)
              (return))
            (:`Is Not Valid`
              (bind _asmc_player_controller (cast `/Game/Blueprints/game/MC_PlayerController` (`GameplayStatics.GetPlayerController` 0)))
              (bind _returnvalue_3 (`|CreateWidget` "/Game/Blueprints/Inventory/InventoryUI/InventoryWidget.InventoryWidget_C" _asmc_player_controller self (`self.InventoryName`)))
              (bind _output_get_2 (set `self.InventoryW` _returnvalue_3))
              (`UserWidget.AddToViewport` _output_get_2 0)
              (set `PlayerController.bShowMouseCursor` true _returnvalue_2)
              (`WidgetBlueprintLibrary.SetInputMode_GameAndUIEx` _returnvalue_2 null)
              (return))))))))