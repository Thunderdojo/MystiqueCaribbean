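; Item_Master is an inventory Blueprint for a world item that characters can pick up.
; Box overlap shows a ScreenMessage widget to the player, removed after a short delay or when overlap ends.
; InterAct adds SlotContent to the character's sack inventory if valid, toggling it twice, otherwise to the action slots with a bar refresh.
; The actor destroys itself after either transfer.
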(event `self.Box.OnComponentBeginOverlap`
  (params (OverlappedComponent :type "PrimitiveComponent Object Reference") (OtherActor :type "Actor Object Reference") (OtherComp :type "PrimitiveComponent Object Reference") (OtherBodyIndex :type Integer) (bFromSweep :type Boolean) (SweepResult :type "HitResult Structure (by ref)"))
  (bind _screenmessage (`self.Screenmessage`))
  (bind _screenmessage_2 (`self.Screenmessage`))
  (if (`.PickedUp?_29_FCEB0BE042117AFCF93E8D916CB6AF13` (break `/Game/Blueprints/Inventory/ItemStruct` (`.ItemStruct_3_38C2D32F4BE57275E6DACCA1553B2273` (break `/Game/Blueprints/Inventory/SlotContent` (`self.SlotContent`)))))
    (`/Engine/EditorBlueprintResources/StandardMacros.IsValid` _screenmessage :!label _label
      (:`Is Valid`
        (`Widget.RemoveFromParent` _screenmessage)
        (set `self.Screenmessage` null)))
    (else
      (`/Engine/EditorBlueprintResources/StandardMacros.IsValid` (`self.Screenmessage`)
        (:`Is Not Valid`
          (bind _asbase_character (cast `/Game/Blueprints/characters/BaseCharacter` OtherActor))
          (set `self.As Base Character` _asbase_character)
          (bind _asmc_player_controller (cast `/Game/Blueprints/game/MC_PlayerController` (`Pawn.GetController` _asbase_character)))
          (bind _returnvalue (`|CreateWidget` "/Game/UI/ScreenMessage.ScreenMessage_C" _asmc_player_controller (`self.Screen Message`) (`self.Letter`)))
          (bind _output_get (set `self.Screenmessage` _returnvalue))
          (`UserWidget.AddToViewport` _output_get 0)
          (`KismetSystemLibrary.Delay` 1.5)
          (`/Engine/EditorBlueprintResources/StandardMacros.IsValid` _screenmessage_2
            (:`Is Valid`
              (`Widget.RemoveFromParent` _screenmessage_2)
              (set `self.Screenmessage` null))))))))

(event `self.Box.OnComponentEndOverlap`
  (params (OverlappedComponent :type "PrimitiveComponent Object Reference") (OtherActor :type "Actor Object Reference") (OtherComp :type "PrimitiveComponent Object Reference") (OtherBodyIndex :type Integer))
  (goto _label))

(event `/Game/Blueprints/interfaces/E_InterFace.InterAct`
  (params (Interactor :type "Actor Object Reference"))
  (`/Engine/EditorBlueprintResources/StandardMacros.IsValid` Interactor
    (:`Is Valid`
      (if (not (`.PickedUp?_29_FCEB0BE042117AFCF93E8D916CB6AF13` (break `/Game/Blueprints/Inventory/ItemStruct` (`.ItemStruct_3_38C2D32F4BE57275E6DACCA1553B2273` (break `/Game/Blueprints/Inventory/SlotContent` (`self.SlotContent`))))))
        (bind _asbase_character (cast `/Game/Blueprints/characters/BaseCharacter` Interactor))
        (set `self.As Base Character` _asbase_character)
        (`/Engine/EditorBlueprintResources/StandardMacros.IsValid` (`/Game/Blueprints/characters/BaseCharacter.SackRef` _asbase_character)
          (:`Is Valid`
            (bind _inventorycomponent (`/Game/Blueprints/Inventory/Sack.InventoryComponent` (`/Game/Blueprints/characters/BaseCharacter.SackRef` _asbase_character)))
            (`/Game/Blueprints/Inventory/InventoryComponent.AddToInventory` _inventorycomponent (`self.SlotContent`))
            (`/Game/Blueprints/Inventory/InventoryComponent.ToggleSack` _inventorycomponent _inventorycomponent)
            (`/Game/Blueprints/Inventory/InventoryComponent.ToggleSack` _inventorycomponent _inventorycomponent)
            (`self.K2_DestroyActor`))
          (:`Is Not Valid`
            (`/Game/Blueprints/Inventory/InventoryComponent.AddToInventory` (`/Game/Blueprints/characters/BaseCharacter.ActionSlots` _asbase_character) (`self.SlotContent`))
            (`/Game/Blueprints/characters/BaseCharacter.RefrreshBAr` _asbase_character)
            (`self.K2_DestroyActor`)))))))

(fn `UserConstructionScript`)