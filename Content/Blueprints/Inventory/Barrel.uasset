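; Barrel is an interactable storage container with a three-slot InventoryComponent.
; Interact drives a FlipFlop that rotates a mesh back and forth and toggles the inventory UI, keeping a widget reference.
; Entering the Box shows a player a screen message for up to one second.
; Leaving removes the message and any valid inventory widget, then calls Shut, which re-enters the same FlipFlop to reverse the toggle.
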(event `self.ReceiveBeginPlay`
  (set `/Game/Blueprints/Inventory/InventoryComponent.NumberOfSlots` 3 (`self.InventoryComponent`)))

(event `self.Box.OnComponentBeginOverlap`
  (params (OverlappedComponent :type "PrimitiveComponent Object Reference") (OtherActor :type "Actor Object Reference") (OtherComp :type "PrimitiveComponent Object Reference") (OtherBodyIndex :type Integer) (bFromSweep :type Boolean) (SweepResult :type "HitResult Structure (by ref)"))
  (bind _screenmessageref (`self.ScreenmessageRef`))
  (bind _asbase_character (cast `/Game/Blueprints/characters/BaseCharacter` OtherActor))
  (bind _asmc_player_controller (cast `/Game/Blueprints/game/MC_PlayerController` (`Pawn.GetController` _asbase_character)))
  (bind _returnvalue (`|CreateWidget` "/Game/UI/ScreenMessage.ScreenMessage_C" _asmc_player_controller))
  (bind _output_get (set `self.ScreenmessageRef` _returnvalue))
  (`UserWidget.AddToViewport` _output_get 0)
  (`KismetSystemLibrary.Delay` 1.0)
  (`/Engine/EditorBlueprintResources/StandardMacros.IsValid` _screenmessageref
    (:`Is Valid`
      (`Widget.RemoveFromParent` _screenmessageref)
      (set `self.ScreenmessageRef` null))))

(event `/Game/Blueprints/interfaces/E_InterFace.InterAct`
  (`/Engine/EditorBlueprintResources/StandardMacros.FlipFlop` :!label _label
    (:`A`
      (`SceneComponent.K2_AddLocalRotation` (`self.StaticMesh1`) (struct :`Pitch` -15.0) false false)
      (bind _inventoryref (`/Game/Blueprints/Inventory/InventoryComponent.ToggleUI` (`self.InventoryComponent`)))
      (set `self.Inventory Ref` _inventoryref))
    (:`B`
      (`SceneComponent.K2_AddLocalRotation` (`self.StaticMesh1`) (struct :`Pitch` 15.0) false false)
      (bind _inventoryref_2 (`/Game/Blueprints/Inventory/InventoryComponent.ToggleUI` (`self.InventoryComponent`)))
      (set `self.Inventory Ref` _inventoryref_2))))

(event `shut`
  (goto _label))

(event `self.Box.OnComponentEndOverlap`
  (params (OverlappedComponent :type "PrimitiveComponent Object Reference") (OtherActor :type "Actor Object Reference") (OtherComp :type "PrimitiveComponent Object Reference") (OtherBodyIndex :type Integer))
  (bind _screenmessageref (`self.ScreenmessageRef`))
  (bind _inventory_ref (`self.Inventory Ref`))
  (cast `/Game/Blueprints/characters/BaseCharacter` OtherActor)
  (`/Engine/EditorBlueprintResources/StandardMacros.IsValid` _screenmessageref
    (:`Is Valid`
      (`Widget.RemoveFromParent` _screenmessageref)
      (set `self.ScreenmessageRef` null))
    (:`Is Not Valid`
      _))
  (`/Engine/EditorBlueprintResources/StandardMacros.IsValid` _inventory_ref
    (:`Is Valid`
      (`Widget.RemoveFromParent` _inventory_ref)
      (set `self.Inventory Ref` null)
      (`self.shut`))))

(fn `UserConstructionScript`)