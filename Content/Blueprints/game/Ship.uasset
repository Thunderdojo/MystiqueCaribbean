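; Ship actor that travels along the spline of a referenced track actor.
; On BeginPlay, if Drive is set, it waits a short delay and then plays the Floatship timeline, with play rate scaled so the trip lasts DurationForMove.
; Each update maps the timeline alpha to a distance along the spline and sets the ship's world location and rotation from it.
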(event `self.ReceiveBeginPlay`
  (if (`self.Drive?`)
    (`self.MoveShip`)))

(event `MoveShip`
  (bind _spline (`/Game/Blueprints/game/Track.Spline` (`self.TrackRef`)))
  (bind _returnvalue (`KismetMathLibrary.Lerp` 0.0 (`SplineComponent.GetSplineLength` _spline) (`self.Alpha`)))
  (`KismetSystemLibrary.Delay` 3.0)
  (`TimelineComponent.SetPlayRate` (`self.Floatship`) (/ 1.0 (`self.DurationForMove`)))
  (bind (_direction _alpha) (`Timeline|Floatship`)
    (:`Update`
      (set `self.Alpha` _alpha)
      (`self.K2_SetActorLocationAndRotation` (`SplineComponent.GetLocationAtDistanceAlongSpline` _spline _returnvalue "World") (`SplineComponent.GetRotationAtDistanceAlongSpline` _spline _returnvalue "World")))))

(fn `UserConstructionScript`)