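; Player controller that sets up the game's UI and input mode on start and handles toggling a map screen.
; On BeginPlay, the Playing flag selects either the in-game HUD with game-only input and hidden cursor, or the main menu with UI-only input and visible cursor.
; The M key creates the Map widget or removes it, using a stored reference as the open/closed state.
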(event `self.ReceiveBeginPlay`
  (`|ExecutionSequence`
    (:`then_0`
      (if (`self.Playing?`)
        (bind _returnvalue (`|CreateWidget` "/Game/UI/IG_Hud.IG_Hud_C"))
        (`UserWidget.AddToViewport` _returnvalue 0)
        (set `self.bShowMouseCursor` false)
        (`/Engine/EditorBlueprintResources/StandardMacros.IsValid` self
          (:`Is Valid`
            (`WidgetBlueprintLibrary.SetInputMode_GameOnly` self)))
        (else
          (bind _returnvalue_2 (`|CreateWidget` "/Game/UI/MainMenu.MainMenu_C"))
          (`UserWidget.AddToViewport` _returnvalue_2 0)
          (set `self.bShowMouseCursor` true)
          (`WidgetBlueprintLibrary.SetInputMode_UIOnlyEx` self _returnvalue_2))))))

(event `Key|M`
  (params (Key :type "Key Structure"))
  (bind _mapref (`self.MapRef`))
  ;[1 1 1] Show map
  (:`Pressed`
    (`/Engine/EditorBlueprintResources/StandardMacros.IsValid` _mapref
      (:`Is Valid`
        (`Widget.RemoveFromParent` _mapref)
        (set `self.MapRef` null))
      (:`Is Not Valid`
        (bind _returnvalue (`|CreateWidget` "/Game/UI/map.map_C"))
        (bind _output_get (set `self.MapRef` _returnvalue))
        (`UserWidget.AddToViewport` _output_get 0)))))

(fn `UserConstructionScript`)